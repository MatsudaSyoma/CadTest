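; Component that moves its owning actor along the spline of a referenced SplineActor.
; On BeginPlay it makes the owner movable, finds its starting spline distance and rotates attached actors based on owner and spline tags.
; Tag handling runs inside a loop over spline tags, so adjustments can repeat, and "Motor" halves Speed per attached actor.
; Tick applies the transform from SplineActor's GetSplineTransform, using frame-scaled speed and a ModifyValue yaw offset.
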(event EventBeginPlay
  (bind _splineactor (Variables|Default|GetSplineActor)
    (:then
      (for _array_element (Variables|/Script/Engine.Actor|GetTags _splineactor)
        (Variables|Default|SetTagName _array_element)
        (Transformation|SetMobility (Variables|/Script/Engine.Actor|GetRootComponent (Components|GetOwner)) "Movable")
        (Variables|Default|SetDistance (Class|SplineComponent|GetDistanceAlongSplineatLocation (Variables|/Game/CADData/No000740_ASSY/BluePrint/BP_Spline.BP_Spline_C|GetSpline (Variables|Default|GetSplineActor)) (Transformation|GetActorLocation (Components|GetOwner)) "World"))
        (for _array_element_2 (Variables|/Script/Engine.Actor|GetTags (Components|GetOwner))
          (if (== _array_element_2 "Modify")
            (for _array_element_3 (Actor|GetAttachedActors (Components|GetOwner) true false)
              (Transformation|SetActorRelativeRotation _array_element_3 "0.000000,180.000000,0.000000"))))
        (for _array_element_4 (Variables|/Script/Engine.Actor|GetTags (Variables|Default|GetSplineActor))
          (if (or (== _array_element_4 "Right") (== _array_element_4 "Motor"))
            (for _array_element_5 (Actor|GetAttachedActors (Components|GetOwner) true false)
              (Transformation|AddActorLocalRotation _array_element_5 "180.000000,0.000000,0.000000" false false)
              (for _array_element_6 (Variables|/Script/Engine.Actor|GetTags (Variables|Default|GetSplineActor))
                (if (== _array_element_6 "Motor")
                  (Variables|Default|SetSpeed (/ (Variables|Default|GetSpeed) 2.0)))))))))
    (:else)))

(event EventTick
  (params (DeltaSeconds :type Float%20%28single-precision%29))
  (Variables|Default|GetSplineActor
    (:then
      (bind _transform (Default|GetSplineTransform (Variables|Default|GetSplineActor) (Variables|Default|GetDistance) (* (Variables|Default|GetSpeed) DeltaSeconds)))
      (Transformation|SetActorTransform (Components|GetOwner) (Math|Transform|MakeTransform (.Location (Math|Transform|BreakTransform _transform)) (Math|Rotator|MakeRotator (.Roll (Math|Rotator|BreakRotator (.Rotation (Math|Transform|BreakTransform _transform)))) (.Pitch (Math|Rotator|BreakRotator (.Rotation (Math|Transform|BreakTransform _transform)))) (+ (.Yaw (Math|Rotator|BreakRotator (.Rotation (Math|Transform|BreakTransform _transform)))) (Variables|Default|GetModifyValue))) (.Scale (Math|Transform|BreakTransform _transform)))))
    (:else)))