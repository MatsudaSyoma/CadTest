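; BP_RotationComponent is a component that continuously spins the actor it is attached to.
; On BeginPlay it sets the owner's root component to Movable so it can rotate at runtime.
; Each tick it applies a local rotation from AddRotator, scaled by delta time and a fixed speed factor, with the Reverse flag flipping the direction.
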(event EventBeginPlay
  (Transformation|SetMobility (Variables|/Script/Engine.Actor|GetRootComponent (Components|GetOwner)) "Movable"))

(event EventTick
  (params (DeltaSeconds :type Float%20%28single-precision%29))
  (Transformation|AddActorLocalRotation (Components|GetOwner) (* (Variables|Default|GetAddRotator) (* DeltaSeconds 22.0 (Math|Float|SelectFloat 1.0 -1.0 (Variables|Default|GetReverse)))) false false))